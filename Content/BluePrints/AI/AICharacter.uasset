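; AI character Blueprint that runs one movement behavior, chosen by AIState at BeginPlay: roam, chase player, patrol or patrol to point.
; Each behavior is a self-restarting AIMoveTo loop that continues only on success.
; Roam picks random nearby navigable points, Patrol chains four fixed target points, and PatrolToPoint cycles through a TargetPoints array by index.
; An explode-and-damage-player sequence is present but unconnected.
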(event `self.ReceiveBeginPlay`
  (switch `/Game/BluePrints/AI/EAIState` (`self.AIState`)
    (:`NewEnumerator1`
      (`self.Roam`))
    (:`NewEnumerator2`
      (`self.ChasePlayer`))
    (:`NewEnumerator3`
      (`self.Patrol`))
    (:`NewEnumerator4`
      (`self.PatrolToPoint`))))

(event `Roam`
  ;[1 1 1] Roaming
  (`|AIMoveTo` self (`NavigationSystem.K2_GetRandomLocationInNavigableRadius` (`self.K2_GetActorLocation`) 500.0)
    (:`OnSuccess`
      (`KismetSystemLibrary.Delay` 1.0)
      (`self.Roam`))))

(event `ChasePlayer`
  ;[1 1 1] Chasing Player
  (`|AIMoveTo` self (0.0 0.0 0.0) (`GameplayStatics.GetPlayerCharacter` 0)
    (:`OnSuccess`
      (`KismetSystemLibrary.Delay` 1.0)
      (`self.ChasePlayer`))))

(event `Patrol`
  ;[1 1 1] Patrol
  (`|AIMoveTo` self (0.0 0.0 0.0) (`self.TargetPoint1`)
    (:`OnSuccess`
      (`KismetSystemLibrary.Delay` 1.0)
      (`|AIMoveTo` self (0.0 0.0 0.0) (`self.TargetPoint2`)
        (:`OnSuccess`
          (`KismetSystemLibrary.Delay` 1.0)
          (`|AIMoveTo` self (0.0 0.0 0.0) (`self.TargetPoint3`)
            (:`OnSuccess`
              (`KismetSystemLibrary.Delay` 1.0)
              (`|AIMoveTo` self (0.0 0.0 0.0) (`self.TargetPoint4`)
                (:`OnSuccess`
                  (`KismetSystemLibrary.Delay` 1.0)
                  (`self.Patrol`))))))))))

(event `PatrolToPoint`
  ;[1 1 1] Patrol(Array)
  (`|AIMoveTo` self (0.0 0.0 0.0) (`|GetArrayItem` (`self.TargetPoints`) (`self.PatrolPointIndex`))
    (:`OnSuccess`
      (if (>= (`self.PatrolPointIndex`) (- (`KismetArrayLibrary.Array_Length` (`self.TargetPoints`)) 1))
        (set `self.PatrolPointIndex` 0)
        (else
          (`/Engine/EditorBlueprintResources/StandardMacros.IncrementInt` (`self.PatrolPointIndex`)
            (:`  `
              _))))
      (`self.PatrolToPoint`))))

(fn `UserConstructionScript`)