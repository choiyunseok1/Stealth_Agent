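; AI enemy character that moves by a state set in AIState and reloads Map1 when it spots the player.
; BeginPlay starts Roam, Chase Player, Patrol or Patrol to Point, each a self-repeating AIMoveTo loop.
; Sight is ignored while the player has UseItem1 or after entering the Sphere, which permanently sets CanBeHacked.
; For hackable AI, EMP with UseItem2 zeroes walk speed briefly, then restarts the state.
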(event `self.ReceiveTick`
  (params (DeltaSeconds :type "Float (single-precision)")))

(event `EMP`
  (bind _charactermovement (`self.CharacterMovement`))
  ;[1 1 1] Using EMP(범위 내에 있는 AI만)
  (if (`self.CanBeHacked`)
    (bind _asmain_character (cast `/Game/BluePrints/BPCharacter/Main_Character` (`GameplayStatics.GetPlayerCharacter` 0)))
    (if (`/Game/BluePrints/BPCharacter/Main_Character.UseItem2` _asmain_character)
      (set `CharacterMovementComponent.MaxWalkSpeed` 0.0 _charactermovement)
      (`KismetSystemLibrary.PrintString` "speed 0" true true (struct :`G` 0.66 :`B` 1.0 :`A` 1.0) 20.0)
      (`KismetSystemLibrary.Delay` 5.0)
      (set `CharacterMovementComponent.MaxWalkSpeed` 300.0 _charactermovement)
      (`KismetSystemLibrary.PrintString` "speed 600" true true (struct :`R` 1.0 :`G` 0.252639 :`B` 0.062211 :`A` 1.0) 20.0)
      (`self.AIStartState`))))

(event `self.ReceiveBeginPlay`
  ;[1 1 1] AI를 작동시킴
  (`self.AIStartState`))

(event `Roam`
  ;[1 1 1] Roaming
  (`|AIMoveTo` self (`NavigationSystem.K2_GetRandomLocationInNavigableRadius` (`self.K2_GetActorLocation`) 500.0)
    (:`OnSuccess`
      (`KismetSystemLibrary.Delay` 1.0)
      (`self.Roam`))))

(event `AIStartState`
  ;[1 1 1] AI State Machine
  (switch `/Game/BluePrints/BPAI/EAIState` (`self.AIState`)
    (:`NewEnumerator1`
      (`self.Roam`))
    (:`NewEnumerator2`
      (`self.ChasePlayer`))
    (:`NewEnumerator3`
      (`self.Patrol`))
    (:`NewEnumerator4`
      (`self.PatrolToPoint`))))

(event `ChasePlayer`
  ;[1 1 1] Chasing Player
  (`|AIMoveTo` self (0.0 0.0 0.0) (`GameplayStatics.GetPlayerCharacter` 0)
    (:`OnSuccess`
      (`KismetSystemLibrary.Delay` 1.0)
      (`self.ChasePlayer`))))

(event `Patrol`
  ;[1 1 1] Patrol
  (`|AIMoveTo` self (0.0 0.0 0.0) (`self.TargetPoint1`)
    (:`OnSuccess`
      (`KismetSystemLibrary.Delay` 1.0)
      (`|AIMoveTo` self (0.0 0.0 0.0) (`self.TargetPoint2`)
        (:`OnSuccess`
          (`KismetSystemLibrary.Delay` 1.0)
          (`|AIMoveTo` self (0.0 0.0 0.0) (`self.TargetPoint3`)
            (:`OnSuccess`
              (`KismetSystemLibrary.Delay` 1.0)
              (`|AIMoveTo` self (0.0 0.0 0.0) (`self.TargetPoint4`)
                (:`OnSuccess`
                  (`KismetSystemLibrary.Delay` 1.0)
                  (`self.Patrol`))))))))))

(event `PatrolToPoint`
  ;[1 1 1] Patrol(Array)
  (`|AIMoveTo` self (0.0 0.0 0.0) (`|GetArrayItem` (`self.TargetPoints`) (`self.PatrolPointIndex`))
    (:`OnSuccess`
      (if (>= (`self.PatrolPointIndex`) (- (`KismetArrayLibrary.Array_Length` (`self.TargetPoints`)) 1))
        (set `self.PatrolPointIndex` 0)
        (else
          (`/Engine/EditorBlueprintResources/StandardMacros.IncrementInt` (`self.PatrolPointIndex`)
            (:`  `
              _))))
      (`self.PatrolToPoint`))))

(event `self.Sphere.OnComponentBeginOverlap`
  (params (OverlappedComponent :type "PrimitiveComponent Object Reference") (OtherActor :type "Actor Object Reference") (OtherComp :type "PrimitiveComponent Object Reference") (OtherBodyIndex :type Integer) (bFromSweep :type Boolean) (SweepResult :type "HitResult Structure (by ref)"))
  ;[1 1 1] EMP Collision에 들어왔는지 확인
  (if (== OtherActor (`GameplayStatics.GetPlayerPawn` 0))
    (`KismetSystemLibrary.PrintString` "overlap player" true true (struct :`R` 0.506594 :`G` 0.092793 :`B` 1.0 :`A` 1.0) 20.0)
    (set `self.CanBeHacked` true)))

(event `self.PawnSensing.OnSeePawn`
  (params (Pawn :type "Pawn Object Reference"))
  ;[1 1 1] Sensing + Restart
  (bind _asmain_character (cast `/Game/BluePrints/BPCharacter/Main_Character` Pawn))
  (if (`/Game/BluePrints/BPCharacter/Main_Character.UseItem1` _asmain_character)
    _
    (elif (not (`self.CanBeHacked`))
      (`GameplayStatics.OpenLevel` "Map1"))))

(fn `UserConstructionScript`)