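; CCTV security camera AI that catches the player on sight, triggering their death and reloading Map1 after a short delay.
; Pawn sensing ignores a Main_Character using item 1, or using item 2 once the camera is hackable; otherwise it also zeroes its own walk speed.
; A sphere overlap, noted as EMP collision, marks the camera hackable when the player enters, and nothing here clears that flag.
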(event `self.PawnSensing.OnSeePawn`
  (params (Pawn :type "Pawn Object Reference"))
  ;[1 1 1] Sensing + Restart
  (bind _asmain_character (cast `/Game/BluePrints/BPCharacter/Main_Character` Pawn))
  (if (`/Game/BluePrints/BPCharacter/Main_Character.UseItem1` _asmain_character)
    _
    (elif (not (and (`/Game/BluePrints/BPCharacter/Main_Character.UseItem2` _asmain_character) (`self.CanBeHacked`)))
      (bind _asmain_character_2 (cast `/Game/BluePrints/BPCharacter/Main_Character` (`GameplayStatics.GetPlayerCharacter` 0)))
      (`/Game/BluePrints/BPCharacter/Main_Character.Death` _asmain_character_2)
      (set `CharacterMovementComponent.MaxWalkSpeed` 0.0 (`self.CharacterMovement`))
      (`KismetSystemLibrary.Delay` 2.0)
      (`GameplayStatics.OpenLevel` "Map1"))))

(event `self.Sphere.OnComponentBeginOverlap`
  (params (OverlappedComponent :type "PrimitiveComponent Object Reference") (OtherActor :type "Actor Object Reference") (OtherComp :type "PrimitiveComponent Object Reference") (OtherBodyIndex :type Integer) (bFromSweep :type Boolean) (SweepResult :type "HitResult Structure (by ref)"))
  ;[1 1 1] EMP Collision에 들어왔는지 확인
  (if (== OtherActor (`GameplayStatics.GetPlayerPawn` 0))
    (`KismetSystemLibrary.PrintString` "cctv overlap player" true true (struct :`R` 0.506594 :`G` 0.092793 :`B` 1.0 :`A` 1.0) 20.0)
    (set `self.CanBeHacked` true)))

(fn `UserConstructionScript`)